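; BP_Torch is a torch with a point light and a fire effect whose shared color reflects goal and clear state.
; The construction script tints both light and fire blue when IsGoal is set.
; On BeginPlay in the "End" level, it turns both red if the AwardGameInstance's IsClear flag is false, overriding any goal tint.
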(event EventBeginPlay
  (bind _returnvalue (Game|GetCurrentLevelName true))
  (if (and (Utilities|Enum|Equal(Enum) _returnvalue "End") (not (Variables|/Game/BP/AwardGameInstance.AwardGameInstance_C|GetIsClear (.AsAward%20Game%20Instance (Utilities|Casting|CastToAwardGameInstance (Game|GetGameInstance))))))
    (Rendering|Components|Light|SetLightColor (Variables|Default|GetPointLight) "(R=1.000000,G=0.000000,B=0.000000,A=1.000000)" true)
    (Effects|Components|ParticleSystem|SetColorParameter (Variables|Default|GetP_Fire) "FireColor" "(R=1.000000,G=0.000000,B=0.000000,A=1.000000)")))

(fn ConstructionScript
  (if (Variables|Default|GetIsGoal)
    (Rendering|Components|Light|SetLightColor (Variables|Default|GetPointLight) "(R=0.019382,G=0.242281,B=1.000000,A=1.000000)" true)
    (Effects|Components|ParticleSystem|SetColorParameter (Variables|Default|GetP_Fire) "FireColor" "(R=0.019382,G=0.242281,B=1.000000,A=1.000000)")))