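; BP_Award is a character controlled by BP_AwardController, with a headlight, point light and one-time death handling.
; On BeginPlay it attaches the audio listener to the headlight and turns both lights red in the "End" level if the game is not cleared.
; The first damage plays a death voice and ragdolls the mesh.
; It then spends a GameInstance life and expires shortly after, or opens "End" when none remain.
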(event EventBeginPlay
  (bind _asbp_award_controller (Utilities|Casting|CastToBP_AwardController (Pawn|GetController))
    (:then
      (Class|PlayerController|SetAudioListenerOverride _asbp_award_controller (Variables|Default|GetHeadLight) "0, 0, 0" "0, 0, 0"))
    (:CastFailed
      _))
  (bind _returnvalue (Game|GetCurrentLevelName true))
  (if (and (Utilities|Enum|Equal(Enum) _returnvalue "End") (not (Variables|/Game/BP/AwardGameInstance.AwardGameInstance_C|GetIsClear (.AsAward%20Game%20Instance (Utilities|Casting|CastToAwardGameInstance (Game|GetGameInstance))))))
    (Rendering|Components|Light|SetLightColor (Variables|Default|GetHeadLight) "(R=1.000000,G=0.000000,B=0.000000,A=1.000000)" true)))

(event Game|Damage|EventAnyDamage
  (params (Damage :type Float%20%28single-precision%29) (DamageType :type Damage%20Type%20Object%20Reference) (InstigatedBy :type Controller%20Object%20Reference) (DamageCauser :type Actor%20Object%20Reference))
  (bind _returnvalue (Game|GetGameInstance))
  (bind _mesh (Variables|Character|GetMesh))
  (bind _asaward_game_instance (Utilities|Casting|CastToAwardGameInstance _returnvalue))
  (bind _life (Variables|/Game/BP/AwardGameInstance.AwardGameInstance_C|GetLife _asaward_game_instance))
  (Utilities|FlowControl|DoOnce false
    (:Completed
      (Audio|PlaySound2D "/Game/Audio/death_voice.death_voice" 1.0 1.0 0.0 0 0)
      (Utilities|FlowControl|Sequence
        (:then_0
          ;[1 1 1] Ragdoll化
          (Development|PrintString "AnyDamage")
          (Pawn|Components|CharacterMovement|DisableMovement (Variables|Character|GetCharacterMovement))
          (Collision|SetCollisionProfileName _mesh "Ragdoll" :!class /Script/Engine.PrimitiveComponent)
          (Physics|SetSimulatePhysics _mesh true))
        (:then_1
          ;[1 1 1] Life減少とレベル遷移処理
          (if (> _life 0)
            (Math|Integer|DecrementInt _life
              (:%20%20
                (Actor|SetLifeSpan 1.0)))
            (else
              (Utilities|FlowControl|Delay 1.0)
              (Game|OpenLevel(byName) "End"))))))))

(fn ConstructionScript)