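; Rock trap actor that launches physics-driven BP_Rock boulders on a looping timer from BeginPlay.
; Each rock spawns offset from the Arrow component and receives a velocity-change impulse along the arrow's forward axis.
; The construction script adds an end hole-wall mesh at HoleWallEndLocation and turns both walls to face each other.
; Rocks that end overlap with the end wall get a very short lifespan, removing them.
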(event OnComponentEndOverlap(HoleWallEndMesh)
  (params (OverlappedComponent :type Primitive%20Component%20Object%20Reference) (OtherActor :type Actor%20Object%20Reference) (OtherComp :type Primitive%20Component%20Object%20Reference) (OtherBodyIndex :type Integer))
  (bind _asbp_rock (Utilities|Casting|CastToBP_Rock OtherActor))
  (Actor|SetLifeSpan _asbp_rock 0.1))

(event Custom|SpawnRock
  (bind _arrow (Variables|Default|GetArrow))
  (bind _returnvalue (Transformation|GetWorldTransform _arrow))
  (bind (_location _rotation _scale) (Math|Transform|BreakTransform _returnvalue))
  (bind _returnvalue_2 (Game|SpawnActorfromClass "/Game/BP/BP_Rock.BP_Rock_C" (Math|Transform|MakeTransform (Math|Transform|TransformLocation _returnvalue "100.000000, 0,-100.000000") _rotation _scale) "Undefined" 0 0))
  (Physics|SetSimulatePhysics (Variables|/Game/BP/BP_Rock.BP_Rock_C|GetRockMesh _returnvalue_2) true)
  (Physics|AddImpulse (Variables|/Game/BP/BP_Rock.BP_Rock_C|GetRockMesh _returnvalue_2) (Math|Transform|TransformDirection (Transformation|GetWorldTransform (Variables|Default|GetArrow)) "500.000000, 0, 0") "None" true))

(event EventBeginPlay
  (Utilities|Time|SetTimerbyEvent (delegate Custom|SpawnRock) 3.0 true))

(fn ConstructionScript
  (bind _holewallendlocation (Variables|Default|GetHoleWallEndLocation))
  (bind _holewallstartmesh (Variables|Default|GetHoleWallStartMesh))
  (bind _relativelocation (Variables|/Script/Engine.SceneComponent|GetRelativeLocation _holewallstartmesh))
  (Transformation|SetRelativeRotation (Variables|Default|GetHoleWallStartMesh) (Math|Rotator|FindLookatRotation _relativelocation _holewallendlocation) false false)
  (bind _returnvalue (AddComponent|AddStaticMeshComponent false (Math|Transform|MakeTransform _holewallendlocation (Math|Rotator|FindLookatRotation _holewallendlocation _relativelocation))))
  (bind _output_get (Variables|Default|SetHoleWallEndMesh _returnvalue))
  (bind _returnvalue_2 (AddComponent|AddArrowComponent false))
  (Transformation|AttachComponentToComponent _returnvalue_2 _output_get "None" "KeepRelative" "KeepRelative" "KeepRelative" false))